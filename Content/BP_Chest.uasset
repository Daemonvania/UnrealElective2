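; Chest Blueprint that opens inventory UI for a chest through its OnOpen event.
; OnOpen creates an inventory chest widget and then a WBP_InventoryExchange widget, passing each the Chest reference and adding both to the viewport.
; Each step shows player 0's mouse cursor and sets UI-only input, so focus is last set to the exchange widget.
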(event `self.OnOpen`
  (params (Chest :type "Chest Object Reference"))
  (bind _returnvalue (`GameplayStatics.GetPlayerController` 0))
  (bind _returnvalue_2 (`GameplayStatics.GetPlayerController` 0))
  (bind _returnvalue_3 (`|CreateWidget` "/Game/WBP_InventoryChest.WBP_InventoryChest_C" _returnvalue_2))
  (set `/Game/WBP_InventoryChest.Chest` Chest _returnvalue_3)
  (`UserWidget.AddToViewport` _returnvalue_3 0)
  (set `PlayerController.bShowMouseCursor` true _returnvalue_2)
  (`WidgetBlueprintLibrary.SetInputMode_UIOnlyEx` _returnvalue_2 _returnvalue_3)
  (bind _returnvalue_4 (`|CreateWidget` "/Game/WBP_InventoryExchange.WBP_InventoryExchange_C" _returnvalue))
  (set `/Game/WBP_InventoryExchange.Chest` Chest _returnvalue_4)
  (`UserWidget.AddToViewport` _returnvalue_4 0)
  (set `PlayerController.bShowMouseCursor` true _returnvalue)
  (`WidgetBlueprintLibrary.SetInputMode_UIOnlyEx` _returnvalue _returnvalue_4))

(fn `UserConstructionScript`)